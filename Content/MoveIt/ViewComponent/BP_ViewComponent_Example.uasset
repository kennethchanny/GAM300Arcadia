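; Example view component for the MoveIt example character that supplies that character's cameras and movement states.
; On BeginPlay it casts and caches the owning BP_MoveIt_ExampleCharacter.
; It returns the character's aim, shooter, over-shoulder, melee and adventure cameras as the state camera list.
; It maps view states like crouch, sprint, floor slide and crouch run to character flags, keeping overlapping states such as sliding and crouch-running distinct.
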(event `self.ReceiveBeginPlay`
  (bind _asbp_move_it_example_character (cast `/MoveIt/Example/BP_MoveIt_ExampleCharacter` (`self.GetOwner`)))
  (set `self.Character` _asbp_move_it_example_character))

(fn `GetCharacterStateCameras`
  (returns (ReturnValue :type "Array of CameraComponent Object Reference"))
  (bind _character (`self.Character`)
    (:`then`
      (return (`|MakeArray` (`/MoveIt/Example/BP_MoveIt_ExampleCharacter.AimCamera` _character) (`/MoveIt/Example/BP_MoveIt_ExampleCharacter.ShooterCamera` _character) (`/MoveIt/Example/BP_MoveIt_ExampleCharacter.OverShoulderCamera` _character) (`/MoveIt/Example/BP_MoveIt_ExampleCharacter.MeleeCamera` _character) (`/MoveIt/Example/BP_MoveIt_ExampleCharacter.AdventureCamera` _character))))
    (:`else`)))

(fn `IsCharacterStateActive`
  (params (State :type Byte))
  (returns (ReturnValue :type Boolean))
  (bind _character (`self.Character`))
  (bind _character_2 (`self.Character`))
  (`self.Character`
    (:`then`
      (switch `/MoveIt/ViewComponent/ECharacterViewState` (cast `/MoveIt/ViewComponent/ECharacterViewState` State)
        (:`NewEnumerator1`
          (return (and (`Character.bIsCrouched` _character) (not (`MICharacter.bIsFloorSliding` _character)) (not (`MICharacter.bIsCrouchRunning` _character)))))
        (:`NewEnumerator2`
          (return (and (`MICharacter.bIsSprinting` _character_2) (not (`MICharacter.bIsCrouchRunning` _character_2)))))
        (:`NewEnumerator3`
          (return (`MICharacter.bIsFloorSliding` (`self.Character`))))
        (:`NewEnumerator4`
          (return (`MICharacter.bIsCrouchRunning` (`self.Character`))))))
    (:`else`
      (return false))))